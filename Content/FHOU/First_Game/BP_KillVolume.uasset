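; BP_KillVolume is a kill zone for the platformer that sends the player character back to a respawn point on contact.
; On box overlap with BP_PlatformingCharacter, it reads CheckPointReached from BP_PlatformingGameMode.
; If set, it moves the character to the first BP_Checkpoint found in the level, otherwise to the first PlayerStart.
; The character is relocated with SetActorLocation rather than destroyed and respawned.
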(event `self.Box.OnComponentBeginOverlap`
  (params (OverlappedComponent :type "PrimitiveComponent Object Reference") (OtherActor :type "Actor Object Reference") (OtherComp :type "PrimitiveComponent Object Reference") (OtherBodyIndex :type Integer) (bFromSweep :type Boolean) (SweepResult :type "HitResult Structure (by ref)"))
  (bind _asbp_platforming_character (cast `/Game/Variant_Platforming/Blueprints/BP_PlatformingCharacter` OtherActor))
  (bind _asbp_platforming_game_mode (cast `/Game/Variant_Platforming/Blueprints/BP_PlatformingGameMode` (`GameplayStatics.GetGameMode`)))
  (if (`/Game/Variant_Platforming/Blueprints/BP_PlatformingGameMode.CheckPointReached` _asbp_platforming_game_mode)
    (bind _outactors (`GameplayStatics.GetAllActorsOfClass` "/Game/FHOU/First_Game/BP_Checkpoint.BP_Checkpoint_C"))
    (`self.K2_SetActorLocation` _asbp_platforming_character (`self.K2_GetActorLocation` (`|GetArrayItem` _outactors)) false false)
    (else
      (bind _outactors_2 (`GameplayStatics.GetAllActorsOfClass` "/Script/Engine.PlayerStart"))
      (`self.K2_SetActorLocation` _asbp_platforming_character (`self.K2_GetActorLocation` (`|GetArrayItem` _outactors_2)) false false))))

(fn `UserConstructionScript`)